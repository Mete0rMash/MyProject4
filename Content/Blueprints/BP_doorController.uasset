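; BP_doorController opens level doors by section index and triggers the win when the final section is reached.
; Its OpenDoor event calls Animate on the matching entry in the Doors array for every index except LastSection.
; For LastSection it instead plays starter music at the player controller's location and calls Win on the FirstPersonHUD.
; Its own Animate function and construction script are empty.
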(event Custom|OpenDoor
  (params (Index :type Integer))
  (if (== Index (Variables|Default|GetlastSection))
    (Audio|PlaySoundatLocation "/Game/StarterContent/Audio/Starter_Music01.Starter_Music01" (Transformation|GetActorLocation (Game|GetPlayerController 0)) "0, 0, 0" 1.0 1.0 0.0 0 0 0)
    (bind _asfirst_person_hud (Utilities|Casting|CastToFirstPersonHUD (HUD|GetHUD (Game|GetPlayerController 0))))
    (Default|Win _asfirst_person_hud)
    (else
      (Default|Animate (Utilities|Array|Get(acopy) (Variables|Default|Getdoors) Index)))))

(fn ConstructionScript)

(fn Animate)